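; BP_MainAsteroid is an asteroid actor with an OWL360Capture component that drifts steadily through the level.
; On BeginPlay it creates the WBP_RT360 widget for the first player and adds it to the viewport.
; Tick moves it along world X at a constant, frame-rate-independent speed without sweeping.
; An unconnected FlipFlop would toggle the capture between EquiRectangular and DomeMaster projection, but never runs.
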(event EventBeginPlay
  (Utilities|FlowControl|Sequence
    (:then_0
      (bind _returnvalue (UserInterface|CreateWidget "/Game/WBP_RT360.WBP_RT360_C" (Game|GetPlayerController 0)))
      (UserInterface|Viewport|AddtoViewport _returnvalue 0))))

(event Collision|EventActorBeginOverlap
  (params (OtherActor :type Actor%20Object%20Reference)))

(event EventTick
  (params (DeltaSeconds :type Float%20%28single-precision%29))
  (Transformation|SetActorLocation (+ (Transformation|GetActorLocation) (* "100.000000,0.000000,0.000000" DeltaSeconds)) false false))

(event Input|KeyboardEvents|A
  (params (Key :type Key%20Structure :default "None")))

(fn ConstructionScript)